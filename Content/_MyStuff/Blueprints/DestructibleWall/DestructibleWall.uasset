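; Destructible wall actor that takes damage, can be healed, shows a health bar widget, and explodes when its health runs out.
; Health queries, Heal and TakeDamage forward to a DamageSystemComponent, whose death and damage-response events are bound in the construction script.
; BeginPlay creates the health bar with the wall as its damageable actor.
; Death spawns an explosion emitter and destroys the actor, while the damage response is empty.
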(event Custom|OnDeath
  (bind _returnvalue (Effects|SpawnEmitteratLocation "/Game/StarterContent/Particles/P_Explosion.P_Explosion" (Transformation|GetActorLocation self)))
  (Class|AssetRegistry|WaitforCompletion(Message) _returnvalue)
  (Actor|DestroyActor self))

(event Custom|DamageResponse
  (params (DamageResponse :type DamageResponse%20Enum :default "NewEnumerator0")))

(event EventBeginPlay
  (bind _returnvalue (UserInterface|CreateWidget "/Game/_MyStuff/Blueprints/DamageSystem/UIW_HealthBar.UIW_HealthBar_C" 0 self))
  (UserInterface|SetWidget (Variables|Default|GetWidget) _returnvalue))

(fn ConstructionScript
  (bind _damagesystemcomponent (Variables|Default|GetDamageSystemComponent))
  (EventDispatchers|BindEventtoOnDeath _damagesystemcomponent (EventDispatchers|CreateEvent :!event Custom|OnDeath))
  (EventDispatchers|BindEventtoOnDamageResponse _damagesystemcomponent (EventDispatchers|CreateEvent :!event Custom|DamageResponse)))

(fn GetCurrentHealth
  (return (Variables|/Game/TopDown/Blueprints/DamageSystemComponent.DamageSystemComponent_C|GetHealth (Variables|Default|GetDamageSystemComponent))))

(fn GetMaxHealth
  (return (Variables|/Game/TopDown/Blueprints/DamageSystemComponent.DamageSystemComponent_C|GetMaxHealth (Variables|Default|GetDamageSystemComponent))))

(fn Heal
  (params (HealAmount :type Float%20%28double-precision%29))
  (bind _newcurrenthealth (Default|Heal (Variables|Default|GetDamageSystemComponent) HealAmount))
  (return _newcurrenthealth))

(fn TakeDamage
  (params (DamageInfo :type Damage%20Info%20Structure))
  (bind _wasdamaged (Default|TakeDamage (Variables|Default|GetDamageSystemComponent) DamageInfo))
  (return _wasdamaged))