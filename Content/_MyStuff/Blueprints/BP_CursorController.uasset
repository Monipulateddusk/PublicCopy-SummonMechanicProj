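; BP_CursorController manages the top-down cursor object, enemy capture selection and cursor-driven camera movement.
; ActivateSelectRegion fires a radial ring of line traces, passing the last unique hit, if a Workshop_C, to the player's capture Blueprint and saving the result on the character.
; Camera events shift the spring arm by normalised, yaw-corrected cursor position within bounds, or by right-mouse drag.
; Helper functions place the cursor under the mouse and apply an accumulated rotation offset.
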(event Custom|CalcMoveCamera
  (bind _returnvalue (Viewport|GetViewportSize))
  (bind _springarmref (Variables|Default|GetSpringArmRef))
  (bind _relativelocation (Variables|/Script/Engine.SceneComponent|GetRelativeLocation _springarmref))
  ;[0 0.1294 1] Get the cursor position in a range between -1 and 1 along both axies. That normalisation will be used to move the camera multiplied by sensitivity
  (bind _returnvalue_2 (Class|WidgetLayoutLibrary|GetMousePositiononViewport))
  (bind _output_get (Variables|Default|SetLastCursorPos _returnvalue_2))
  (bind _normalised_output (CallFunction|GetNormalisation (.x _output_get) 0.0 (.x _returnvalue))) ; X-Axis Normalisation
  (bind _normalised_output_2 (CallFunction|GetNormalisation (.y _output_get) 0.0 (.y _returnvalue))) ; Y-Axis Normalisation
  ;[1 0.009047 0.5682] If the player is flipped 180 degrees on the Z axis, invert the camera movement so that it doesn't flip the camera controls
  (if (>= (Math|Float|Absolute(Float) (.yaw (.rotation (Transformation|GetActorTransform (Variables|Components|GetTopDownCharRef))))) 45.0)
    (Transformation|AddRelativeLocation (Variables|Default|GetSpringArmRef) (* (Math|Vector|MakeVector (* _normalised_output_2 (Variables|Default|GetSensitivity)) (* _normalised_output (* (Variables|Default|GetSensitivity) -1.0)) 0.0) "-1.000000,-1.000000,0.000000") false false)
    (else
      (Transformation|AddRelativeLocation (Variables|Default|GetSpringArmRef) (Math|Vector|MakeVector (* _normalised_output_2 (Variables|Default|GetSensitivity)) (* _normalised_output (* (Variables|Default|GetSensitivity) -1.0)) 0.0) false false)))
  ;[0 0.1294 1] Clamp the camera to predefined bounds
  (Transformation|SetRelativeLocation (Variables|Default|GetSpringArmRef) (Math|Vector|MakeVector (Math|Float|Clamp(Float) (.x _relativelocation) -3.5e+02 3.5e+02) (Math|Float|Clamp(Float) (.y _relativelocation) -3.5e+02 3.5e+02) 0.0) false false))

(event Custom|ActivateSelectRegion
  (params (CursorLocation :type Vector))
  (bind _returnvalue (+ CursorLocation "0.000000,0.000000,20.000000"))
  (bind _bp_cursorobject (Variables|Default|GetBP_CursorObject))
  (bind _hitresults (Variables|Default|GetHitResults))
  ;[1 0 0.709] Get where the cursor is and make a ring of influence around it with a fixed radius
  (Utilities|Array|Clear (Variables|Default|GetHitResults))
  (Rendering|SetVisibility _bp_cursorobject true false)
  (Transformation|SetWorldLocation _bp_cursorobject CursorLocation false false)
  (if true
    (for _index (range 0 (Variables|Default|GetNumRaycasts))
      (bind (_outhit _returnvalue_2) (Collision|LineTraceByChannel _returnvalue (+ _returnvalue (* (Math|Vector|RotateVector (Math|Vector|GetForwardVector "0.000000,0.000000,1.000000") (Math|Rotator|MakeRotator 0.0 0.0 (* _index (Variables|Default|GetAngleDegree)))) (Variables|Default|GetRadius))) "TraceTypeQuery3" false 0 "None"))
      (if _returnvalue_2
        (if (not (Utilities|Array|ContainsItem (Variables|Default|GetHitResults) _outhit))
          (Utilities|Array|Add (Variables|Default|GetHitResults) _outhit))))
    ;[0 0.001495 1] Get the last index of the hit results, if it is a workshop_c (the enemy we can capture), then send that data to the capture enemy function in the capture BP
    (if (Utilities|Array|IsNotEmpty _hitresults)
      (bind _asworkshop_c (Utilities|Casting|CastToWorkshop_C (.HitActor (Collision|BreakHitResult (Utilities|Array|Get(acopy) _hitresults (Utilities|Array|LastIndex _hitresults))))))
      (Development|PrintString "FOUND WORKSHOP C")
      (bind _output (Default|FCaptureEnemy (Variables|/Game/TopDown/Blueprints/BP_TopDownCharacter.BP_TopDownCharacter_C|GetPlayerCapture_BP (Variables|Components|GetTopDownCharRef)) _asworkshop_c))
      (Default|SaveEnemyDatatoLocals (Variables|Components|GetTopDownCharRef) _output))))

(event Custom|MoveCamera
  ;[1 1 1] Taking the cursor positions relative to the screen and moving  the camera to the position
  (if (Game|Player|IsInputKeyDown (Game|GetPlayerController 0) "RightMouseButton")
    (bind _returnvalue (Class|WidgetLayoutLibrary|GetMousePositiononViewport))
    (Variables|Default|SetNewCursorPos _returnvalue)
    (Transformation|AddWorldOffset (Variables|Default|GetSpringArmRef) (Math|Vector|MakeVector (* (.x (- (Variables|Default|GetNewCursorPos) (Variables|Default|GetLastCursorPos))) (* (Variables|Default|GetSensitivity) -1.0)) (* (.y (- (Variables|Default|GetNewCursorPos) (Variables|Default|GetLastCursorPos))) (Variables|Default|GetSensitivity)) 0.0) false false)
    (Variables|Default|SetLastCursorPos (Variables|Default|GetNewCursorPos))))

(event EventBeginPlay
  ;[1 1 1] Getting the player character and storing a referance to it
  (bind _asbp_top_down_character (Utilities|Casting|CastToBP_TopDownCharacter (Game|GetPlayerCharacter 0))
    (:then
      (Variables|Components|SetTopDownCharRef _asbp_top_down_character))
    (:CastFailed
      (Development|PrintString "UNABLE TO GET TOP DOWN CHAR"))))

(fn GetLocationUnderCursor
  (params (AccountForWorkshop_COrigin? :type Boolean))
  (bind _returnvalue (Game|GetPlayerController 0))
  (bind _hitresult (Game|Player|GetHitResultUnderCursorbyChannel _returnvalue "TraceTypeQuery1" true))
  (bind (_bblockinghit _binitialoverlap _time _distance _location) (Collision|BreakHitResult _hitresult))
  (if AccountForWorkshop_COrigin?
    (return _bblockinghit (+ "0.000000,0.000000,90.000000" _location))
    (else
      (return _bblockinghit _location))))

(fn GetNormalisation
  (params (value_ :type Float%20%28double-precision%29) (minimum_ :type Float%20%28double-precision%29) (maximum_ :type Float%20%28double-precision%29))
  (return (- (* (/ (- value_ minimum_) (- minimum_ maximum_)) 2.0) -1.0)))

(fn UpdateCursorPosition
  (bind _bp_cursorobject (Variables|Default|GetBP_CursorObject))
  (Rendering|SetVisibility _bp_cursorobject true false)
  (bind (_hit _location_) (CallFunction|GetLocationUnderCursor false))
  (if _hit
    (Transformation|SetWorldLocation _bp_cursorobject _location_ false false)
    (return _location_)))

(fn UpdateCursorRotation
  (params (InputRotation :type Rotator))
  (bind _rotationoffset (Variables|Default|GetRotationOffset))
  (bind _returnvalue (Math|Rotator|CombineRotators InputRotation _rotationoffset))
  (Transformation|SetWorldRotation (Variables|Default|GetBP_CursorObject) _returnvalue false false)
  (return _returnvalue))

(fn ClearRotationOffset
  (Variables|Default|SetRotationOffset "0, 0, 0"))

(fn IncrementRotationOffset
  (params (IncremationOffset :type Rotator))
  (Variables|Default|SetRotationOffset (Math|Rotator|CombineRotators IncremationOffset (Variables|Default|GetRotationOffset))))