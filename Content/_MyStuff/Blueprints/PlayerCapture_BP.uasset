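; PlayerCapture_BP lets the player capture an enemy and spawn and place a new one.
; FCaptureEnemy calls OnCapture on the target and returns its output if valid.
; With a valid montage in SpawnDataOfEnemy, SpawnEnemy creates one Workshop actor, locking further spawns while UpdateEnemyReferance repositions it.
; ApplySpawnDataToSpawnedEnemy sets its final transform, montage and animation start, initialises it, then unlocks spawning.
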(event Custom|SpawnEnemy
  (params (Location :type Vector) (Rotation :type Rotator) (SpawnDataOfEnemy :type Spawn%20Data%20Structure))
  ;[1 1 1] When Activated, spawn an enemy and store that spawned enemy as a referance so we can edit the position + rotation. Prevent future spawning
  (if (and (Utilities|IsValid (.montage_to_play SpawnDataOfEnemy)) (not (Variables|Default|GetIsNotAbleToSpawnEnemy?)))
    (bind _returnvalue (Game|SpawnActorfromClass :Class "/Game/_MyStuff/Blueprints/Workshop_C.Workshop_C_C" :SpawnTransform (Math|Transform|MakeTransform Location Rotation) :CollisionHandlingOverride "Undefined" :TransformScaleMethod "MultiplyWithRoot" :Instigator 0))
    (Variables|Default|SetEnemyReferance _returnvalue)
    (Variables|Default|SetIsNotAbleToSpawnEnemy? true)))

(event Custom|UpdateEnemyReferance
  (params (Location :type Vector) (Rotation :type Rotator))
  (bind _enemyreferance (Variables|Default|GetEnemyReferance))
  ;[1 1 1] Update the position and rotation of the enemy referance
  (if (and (Utilities|IsValid _enemyreferance) (Variables|Default|GetIsNotAbleToSpawnEnemy?))
    (Transformation|SetActorTransform _enemyreferance (Math|Transform|MakeTransform Location Rotation))))

(event Custom|ApplySpawnDataToSpawnedEnemy
  (params (Location :type Vector) (Rotation :type Rotator) (Animation_Start_Duration :type Float%20%28double-precision%29) (Montage_To_Play :type Anim%20Montage%20Object%20Reference))
  (bind _enemyreferance (Variables|Default|GetEnemyReferance))
  ;[1 1 1] Initalise the enemy referance. Allow a new enemy to be spawned
  (if (Utilities|IsValid Montage_To_Play)
    (CallFunction|UpdateEnemyReferance Location Rotation)
    (Variables|/Game/_MyStuff/Blueprints/Workshop_C.Workshop_C_C|SetSpawnData _enemyreferance (Utilities|Struct|MakeSpawnData Animation_Start_Duration Montage_To_Play))
    (Default|InitialiseCharacter _enemyreferance)
    (Variables|Default|SetIsNotAbleToSpawnEnemy? false)))

(event EventTick
  (params (DeltaSeconds :type Float%20%28single-precision%29)))

(fn FCaptureEnemy
  (params (EnemyToCapture :type Workshop%20C%20Object%20Reference))
  ;[1 1 1] On this event firing, capture the enemy only if the enemy to capture is valid. Store that data locally
  (if (Utilities|IsValid EnemyToCapture)
    (bind (_isvalidcapture_ _output) (Default|OnCapture EnemyToCapture))
    (if _isvalidcapture_
      (return _output)
      (else
        _)))
  (Development|PrintString "NOT VALID ENEMY TO CAPTURE"))