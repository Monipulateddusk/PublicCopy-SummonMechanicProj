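; Damageable melee character that can be captured mid-montage and spawned as a summon that replays it from the saved position, then destroys itself on completion.
; DoSwitchBoolean alternates heavy and light attack montages.
; Montage notify names select hand or foot sockets for sphere traces, sending damage to hit actors and spawning explosions.
; DamageSystemComponent handles health behind wrapper functions and a health bar widget, while death and damage-response events are empty.
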(event Custom|DoSwitchBoolean
  (bind _output_get (Variables|Default|SetIsDoingHeavyAttack (not (Variables|Default|GetIsDoingHeavyAttack))))
  (if _output_get
    (bind _notifyname (Animation|Montage|PlayMontage (Variables|Character|GetMesh) (Variables|Default|GetHeavyAttackMontageRef))
      (:OnNotifyBegin
        (bind (_outhit _returnvalue _endposition) (Utilities|SpawnSphereTraceatBoneLocation _notifyname))
        (if _returnvalue
          (bind _wasdamaged (Class|IDamagable|TakeDamage(Message) (.HitActor (Collision|BreakHitResult _outhit)) (Utilities|Struct|MakeDamageInfo 15.0 "NewEnumerator1" "NewEnumerator1" true)))
          (if _wasdamaged
            (Effects|SpawnEmitteratLocation "/Game/StarterContent/Particles/P_Explosion.P_Explosion" _endposition)))))
    (else
      (bind _notifyname_2 (Animation|Montage|PlayMontage (Variables|Character|GetMesh) (Variables|Default|GetLightAttackMontageRef))
        (:OnNotifyBegin
          (bind (_outhit_2 _returnvalue_2 _endposition_2) (Utilities|SpawnSphereTraceatBoneLocation _notifyname_2))
          (if _returnvalue_2
            (bind _wasdamaged_2 (Class|IDamagable|TakeDamage(Message) (.HitActor (Collision|BreakHitResult _outhit_2)) (Utilities|Struct|MakeDamageInfo 2.5 "NewEnumerator1" "NewEnumerator1" true)))
            (if _wasdamaged_2
              (Effects|SpawnEmitteratLocation "/Game/StarterContent/Particles/P_Explosion.P_Explosion" _endposition_2))))))))

(event Custom|InitialiseCharacter
  (bind _spawndata (Variables|Default|GetSpawnData))
  ;[1 1 1] Called within the SpawnerBP used when spawning the summoned actor getting over the timing issue of on event start
  (bind _notifyname (Animation|Montage|PlayMontage (Variables|Character|GetMesh) (.montage_to_play _spawndata) 1.0 (.animation_start_duration _spawndata))
    (:OnCompleted
      (Actor|DestroyActor))
    (:OnNotifyBegin
      (bind (_outhit _returnvalue _endposition) (Utilities|SpawnSphereTraceatBoneLocation _notifyname))
      (if _returnvalue
        (bind _wasdamaged (Class|IDamagable|TakeDamage(Message) (.HitActor (Collision|BreakHitResult _outhit)) (Utilities|Struct|MakeDamageInfo 15.0 "NewEnumerator1" "NewEnumerator1" true)))
        (if _wasdamaged
          (Effects|SpawnEmitteratLocation "/Game/StarterContent/Particles/P_Explosion.P_Explosion" _endposition))))))

(event Custom|OnDeath)

(event Custom|DamageResponse
  (params (DamageResponse :type DamageResponse%20Enum :default "NewEnumerator0")))

(event EventBeginPlay
  (bind _returnvalue (UserInterface|CreateWidget "/Game/_MyStuff/Blueprints/DamageSystem/UIW_HealthBar.UIW_HealthBar_C" 0 self))
  (UserInterface|SetWidget (Variables|Default|GetWidget) _returnvalue))

(fn ConstructionScript
  (bind _damagesystemcomponent (Variables|Default|GetDamageSystemComponent))
  (EventDispatchers|BindEventtoOnDeath _damagesystemcomponent (EventDispatchers|CreateEvent :!event Custom|OnDeath))
  (EventDispatchers|BindEventtoOnDamageResponse _damagesystemcomponent (EventDispatchers|CreateEvent :!event Custom|DamageResponse)))

(fn OnCapture
  (bind _mesh (Variables|Character|GetMesh))
  (bind _returnvalue (Components|SkeletalMesh|GetAnimInstance _mesh))
  (bind _returnvalue_2 (Animation|Montage|GetCurrentActiveMontage _returnvalue))
  (return (Utilities|IsValid _returnvalue_2) (Utilities|Struct|MakeSpawnData (Animation|Montage|MontageGetPosition _returnvalue _returnvalue_2) _returnvalue_2)))

(fn GetBoneLocationfromMontageNotifyName
  (params (NotifyName :type Name))
  (switch name NotifyName
    (:Kick
      (return (Transformation|GetSocketLocation (Variables|Character|GetMesh) "foot_r")))
    (:PunchR
      (return (Transformation|GetSocketLocation (Variables|Character|GetMesh) "hand_r")))
    (:PunchL
      (return (Transformation|GetSocketLocation (Variables|Character|GetMesh) "hand_l")))))

(fn GetCurrentHealth
  (return (Variables|/Game/TopDown/Blueprints/DamageSystemComponent.DamageSystemComponent_C|GetHealth (Variables|Default|GetDamageSystemComponent))))

(fn GetMaxHealth
  (return (Variables|/Game/TopDown/Blueprints/DamageSystemComponent.DamageSystemComponent_C|GetMaxHealth (Variables|Default|GetDamageSystemComponent))))

(fn Heal
  (params (HealAmount :type Float%20%28double-precision%29))
  (bind _newcurrenthealth (Default|Heal (Variables|Default|GetDamageSystemComponent) HealAmount))
  (return _newcurrenthealth))

(fn TakeDamage
  (params (DamageInfo :type Damage%20Info%20Structure))
  (bind _wasdamaged (Default|TakeDamage (Variables|Default|GetDamageSystemComponent) DamageInfo))
  (return _wasdamaged))